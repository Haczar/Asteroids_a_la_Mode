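; Ship-fired projectile for a two-player asteroid shooter that scores hits and lives for about one second.
; It increments the instigator Ship's missile count on spawn, while Tick times its lifetime.
; KillYurself awards points by asteroid size through DebugState to the player identified by PlyrName, then decrements the count and destroys the actor.
; A local GivePoints function duplicates scoring with debug prints but is not called here.
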(event Custom|Kill%20Yurself
  (params (Object%20Collided :type Object%20Object%20Reference))
  (bind _returnvalue (Game|GetInstigator))
  (bind _returnvalue_2 (Game|GetGameState))
  (bind _asdebug_state (Utilities|Casting|CastToDebugState _returnvalue_2))
  (bind _asplyr_state (Utilities|Casting|CastToPlyrState (Variables|/Script/Engine.Pawn|GetPlayerState _returnvalue))
    (:then
      (if (Utilities|Name|Equal(Name) (Variables|/Game/Player/PlyrState.PlyrState_C|GetPlyr%20Name _asplyr_state) "Player One")
        _
        (else
          _))
      (Utilities|Casting|CastToAsteroid_Large Object%20Collided
        (:then
          (Default|GivePoints _asdebug_state (Utilities|Name|Equal(Name) (Variables|/Game/Player/PlyrState.PlyrState_C|GetPlyr%20Name _asplyr_state) "Player One") 20))
        (:CastFailed
          (Utilities|Casting|CastToAsteroid_Medium Object%20Collided
            (:then
              (Default|GivePoints _asdebug_state (Utilities|Name|Equal(Name) (Variables|/Game/Player/PlyrState.PlyrState_C|GetPlyr%20Name _asplyr_state) "Player One") 50))
            (:CastFailed
              (Utilities|Casting|CastToAsteroid_Small Object%20Collided
                (:then
                  (Default|GivePoints _asdebug_state (Utilities|Name|Equal(Name) (Variables|/Game/Player/PlyrState.PlyrState_C|GetPlyr%20Name _asplyr_state) "Player One") 100))
                (:CastFailed
                  _)))))))
    (:CastFailed
      _))
  (bind _asship (Utilities|Casting|CastToShip _returnvalue))
  (Math|Integer|DecrementInt (Variables|/Game/Ship/Ship.Ship_C|GetMissleCount _asship)
    (:%20%20
      (Actor|DestroyActor))))

(event EventBeginPlay
  (bind _asship (Utilities|Casting|CastToShip (Game|GetInstigator)))
  (Math|Integer|IncrementInt (Variables|/Game/Ship/Ship.Ship_C|GetMissleCount _asship)))

(event EventTick
  (params (DeltaSeconds :type Float%20%28single-precision%29))
  (bind _output_get (Variables|Default|SetTimeElapsed (+ DeltaSeconds (Variables|Default|GetTimeElapsed))))
  (if (>= _output_get 1.0)
    (CallFunction|KillYurself)))

(fn ConstructionScript)

(fn GivePoints
  (params (P1? :type Boolean) (Points%20Amount :type Integer))
  (bind _asdebug_state (Utilities|Casting|CastToDebugState (Game|GetGameState)))
  (if P1?
    (bind _output_get (Variables|/Game/Modes/Debug/DebugState.DebugState_C|SetScoreP1 _asdebug_state (+ (Variables|/Game/Modes/Debug/DebugState.DebugState_C|GetScoreP1 _asdebug_state) Points%20Amount)))
    (Development|PrintString "Player 1 Points: ")
    (Development|PrintString (Utilities|String|ToString(Integer) _output_get))
    (else
      (bind _output_get_2 (Variables|/Game/Modes/Debug/DebugState.DebugState_C|SetScoreP2 _asdebug_state (+ (Variables|/Game/Modes/Debug/DebugState.DebugState_C|GetScoreP2 _asdebug_state) Points%20Amount)))
      (Development|PrintString "Player 2 Points: ")
      (Development|PrintString (Utilities|String|ToString(Integer) _output_get_2)))))