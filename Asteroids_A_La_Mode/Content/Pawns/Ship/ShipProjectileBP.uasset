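; Ship-fired projectile that tracks its count on the instigating ship and scores asteroid hits for its player.
; BeginPlay increments the ship's MissleCount, and the Destroyed path decrements it and calls DestroyActor.
; HandleAsteroidCollision identifies Player One by the owner's PlayerState name, then a macro awards size-based points through the DebugMData game state, more for smaller asteroids.
; All collision outcomes, including failed casts, feed into the Destroyed path.
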(event EventBeginPlay
  (bind _asship (Utilities|Casting|CastToShip (Game|GetInstigator))
    (:then
      (Math|Integer|IncrementInt (Variables|/Game/Pawns/Ship/Ship.Ship_C|GetMissleCount _asship)))
    (:CastFailed
      (Development|PrintString "failed to cast to ship"))))

(event EventHandleAsteroidCollision
  (params (AsteroidObj :type Object%20Object%20Reference))
  (bind _asuser_data (Utilities|Casting|CastToUserData (Variables|/Script/Engine.Controller|GetPlayerState (.AsReg%20User (Utilities|Casting|CastToRegUser (Components|GetOwner)))))
    (:then
      (|DealwithAsteroidCollision (.AsDebug%20MData (Utilities|Casting|CastToDebugMData (Game|GetGameState))) AsteroidObj (Utilities|Name|Equal(Name) (Variables|/Game/Player/UserData.UserData_C|GetPlyr%20Name _asuser_data) "Player One")
        (:Points%20for%20Large%20Given
          _)
        (:Points%20for%20Medium%20Given
          _)
        (:Points%20for%20Small%20Given
          _)
        (:Fail%20to%20cast%20to%20a%20reconizable%20object.
          _)))
    (:CastFailed
      (Development|PrintString "Failed to cast to user.")))
  (bind _asship (Utilities|Casting|CastToShip (Game|GetInstigator))
    (:then
      (Math|Integer|DecrementInt (Variables|/Game/Pawns/Ship/Ship.Ship_C|GetMissleCount _asship)
        (:%20%20
          (Actor|DestroyActor))))
    (:CastFailed
      (Development|PrintString "Failed to cast to chip"))))

(event EventDestroyed
  (bind _asship (Utilities|Casting|CastToShip (Game|GetInstigator))
    (:then
      (Math|Integer|DecrementInt (Variables|/Game/Pawns/Ship/Ship.Ship_C|GetMissleCount _asship)
        (:%20%20
          (Actor|DestroyActor))))
    (:CastFailed
      (Development|PrintString "Failed to cast to chip"))))

(fn ConstructionScript)