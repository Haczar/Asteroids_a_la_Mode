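; BP_BulletProjectile is a bullet actor that destroys itself after a short lifetime or on contact with another bullet of the same class.
; Its Box overlap casts the other actor to BP_BulletProjectile and ignores anything else.
; On a match, both bullets run SpawnPopoutBullet, which spawns a PopoutBullet at the static mesh's transform and destroys the projectile.
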(event OnComponentBeginOverlap(Box)
  (params (OverlappedComponent :type Primitive%20Component%20Object%20Reference) (OtherActor :type Actor%20Object%20Reference) (OtherComp :type Primitive%20Component%20Object%20Reference) (OtherBodyIndex :type Integer) (bFromSweep :type Boolean) (SweepResult :type Hit%20Result%20Structure%20%28by%20ref%29))
  ;[1 1 1] Bullet Collision
  (if (!= OtherActor self)
    (bind _asbp_bullet_projectile (Utilities|Casting|CastToBP_BulletProjectile OtherActor))
    (CallFunction|SpawnPopoutBullet _asbp_bullet_projectile)
    (CallFunction|SpawnPopoutBullet)))

(event EventBeginPlay
  ;[1 1 1] Auto Destroy Bullet
  (Utilities|FlowControl|Delay 5.0)
  (Actor|DestroyActor))

(fn ConstructionScript)

(fn SpawnPopoutBullet
  (Game|SpawnActorfromClass "/Game/Z_Folder/Blueprints/Weapon/PopoutBullet.PopoutBullet_C" (Transformation|GetWorldTransform (Variables|Default|GetStaticMesh)) "Undefined" 0 0)
  (Actor|DestroyActor))