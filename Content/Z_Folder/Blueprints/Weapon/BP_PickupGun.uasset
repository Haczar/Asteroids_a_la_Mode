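; BP_PickupGun is a gun actor that the motion controller can pick up and that returns to a holster socket when dropped.
; Pickup snaps the root component to the "gun_hold" socket of the component passed in by BP_MotionController.
; Drop detaches the actor and snaps it back onto a stored character mesh socket, so it uses attachment alone in both states.
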(event EventPickup
  (params (AttachTo :type Scene%20Component%20Object%20Reference))
  (|Pickupgun AttachTo))

(event EventDrop
  (|Putgunback))

(fn ConstructionScript)